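; Demo actor for a dash VFX that moves a skeletal mesh along a spline in a repeating slow-then-dash cycle.
; The MoveSlow timeline sets normalized spline distance; when it finishes, Niagara activates, the run animation plays and MoveCharecter adds its track value to that distance every update.
; Both phases align the mesh to the spline with a yaw offset.
; When the dash ends, Niagara deactivates and MoveSlow restarts.
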(event `self.ReceiveBeginPlay`
  (bind _spline (`self.Spline`))
  (bind _returnvalue (* (`self.Distance`) (`SplineComponent.GetSplineLength` (`self.Spline`))))
  (bind (_returnvalue_roll _returnvalue_pitch _returnvalue_yaw) (`KismetMathLibrary.BreakRotator` (`SplineComponent.GetRotationAtDistanceAlongSpline` _spline _returnvalue "Local")))
  (bind (_direction _newtrack_0) (`Timeline|MoveSlow` :!via `PlayFromStart` :!label _label)
    (:`Update`
      (set `self.Distance` _newtrack_0))
    (:`Finished`
      (`ActorComponent.Activate` (`self.Niagara`) true)
      (`SkeletalMeshComponent.PlayAnimation` (`self.SkeletalMesh`) "/Game/AdvancedDashVFX/DemoContent/Mannequin/Animations/ThirdPersonRun.ThirdPersonRun" true)
      (bind (_direction_2 _distance) (`Timeline|MoveCharecter` :!via `PlayFromStart`)
        (:`Update`
          (set `self.Distance` (+ (`self.Distance`) _distance)))
        (:`Finished`
          (`SkeletalMeshComponent.PlayAnimation` (`self.SkeletalMesh`) "/Game/AdvancedDashVFX/DemoContent/Mannequin/Animations/ThirdPersonRun.ThirdPersonRun" true)
          (`ActorComponent.Deactivate` (`self.Niagara`))
          (goto _label :!via `PlayFromStart`)))))
  (`SceneComponent.K2_SetWorldLocation` (`self.SkeletalMesh`) (`SplineComponent.GetLocationAtDistanceAlongSpline` _spline _returnvalue "World") false false)
  (`SceneComponent.K2_SetRelativeRotation` (`self.SkeletalMesh`) (`KismetMathLibrary.MakeRotator` _returnvalue_roll _returnvalue_pitch (+ _returnvalue_yaw -90.0)) false false))

(fn `UserConstructionScript`)