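; Legacy single-player flight component that gives its owning Character Hover and Fast Flight modes.
; Toggle functions swap movement settings; Fast Flight shrinks the capsule, traces for room before restoring it, and exits preserve some vertical momentum.
; Tick eases rotation toward control rotation, derives lean rates for animation and applies decaying dodge forces.
; Steep impacts during Fast Flight switch to Hover on walls or trigger a movement-locking ground slam on floors.
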(event `self.ReceiveBeginPlay`
  (bind _movementcomponent (`self.MovementComponent`))
  ;[0.599 1 0.6833] Save references to the character, its capsule component, and its movement component.
  (bind _ascharacter (cast `Character` (`self.GetOwner`)))
  (set `self.Character` _ascharacter)
  (set `self.MovementComponent` (`Character.CharacterMovement` _ascharacter))
  (bind _output_get (set `self.CapsuleComponent` (`Character.CapsuleComponent` _ascharacter)))
  ;[0.599 1 0.6833] Record starting capsule size. Used to check if there's enough room, and restore the original capsule height, when exiting FastFlight.
  (set `self.CapsuleHalfHeight` (`CapsuleComponent.GetUnscaledCapsuleHalfHeight` _output_get))
  (set `self.CapsuleRadius` (`CapsuleComponent.GetUnscaledCapsuleRadius` _output_get))
  ;[0.599 1 0.6833] Record the character's starting/ground acceleration so it can be restored when flight modes end.
  (set `self.DefaultAcceleration` (`CharacterMovementComponent.MaxAcceleration` _movementcomponent))
  ;[0.599 1 0.6833] Set flight deceleration to the parameter's value.
  (set `CharacterMovementComponent.BrakingDecelerationFlying` (`self.AirBraking`) _movementcomponent)
  ;[0.599 1 0.6833] If a Hit event triggers on the character, run a custom event here.
  (add `Actor.OnActorHit` (`self.Character`) (delegate `Hit`)))

(event `Hit`
  (params (SelfActor :type "Actor Object Reference") (OtherActor :type "Actor Object Reference") (NormalImpulse :type "Vector Structure") (Hit :type "HitResult Structure (by ref)"))
  (bind (_bblockinghit _binitialoverlap _time _distance _location _impactpoint _normal _impactnormal) (`GameplayStatics.BreakHitResult` Hit))
  ;[0.599 1 0.6833] If the player hits a surface at a sharp angle ( >150 degrees), Fast Flight is canceled
  (if (and (> (`KismetMathLibrary.DegAcos` (`KismetMathLibrary.Dot_VectorVector` (`SceneComponent.GetForwardVector` (`self.CapsuleComponent`)) _impactnormal)) 125.0) (`self.FastFlight`))
    ;[0.599 1 0.6833] If the surface impacted is a floor, disable flight to land on it. Otherwise, switch to hover mode.
    (if (< (.z _impactnormal) 0.5)
      (`self.ToggleHover`)
      (else
        (`self.ToggleFastFlight`)
        ;[0.599 1 0.6833] If FastFlight was disabled successfully when impacting the floor, trigger the ground slam.
        (if (not (`self.FastFlight`))
          (`self.TriggerGroundSlam`))))))

(event `self.ReceiveTick`
  (params (DeltaSeconds :type "Float (single-precision)"))
  ;[0.599 1 0.6833] Call the FlightUpdates event each tick to update flight behaviors (that aren't driven by Movement Input)
  (set `self.Delta` DeltaSeconds)
  (`self.FlightUpdates`))

(event `FlightUpdates`
  (bind _returnvalue (`Pawn.GetControlRotation` (`self.Character`)))
  (bind (_returnvalue_roll _returnvalue_pitch _returnvalue_yaw) (`KismetMathLibrary.BreakRotator` (`SceneComponent.K2_GetComponentRotation` (`self.CapsuleComponent`))))
  (bind _returnvalue_2 (`KismetMathLibrary.GetRightVector` (`Pawn.GetControlRotation` (`self.Character`))))
  ;[0.599 1 0.6833] Updates flight logic if either flight mode is active.
  (if (or (`self.Hover`) (`self.FastFlight`))
    (`Actor.K2_SetActorRotation` (`self.Character`) (`KismetMathLibrary.RInterpTo` (`SceneComponent.K2_GetComponentRotation` (`self.CapsuleComponent`)) (select `bool` (`self.Hover`) :`false` _returnvalue :`true` (`KismetMathLibrary.MakeRotator` (.roll _returnvalue) 0.0 (.yaw _returnvalue))) (`self.Delta`) 8.0) false)
    (bind _returnvalue_3 (`PrimitiveComponent.GetPhysicsAngularVelocityInDegrees` (`self.CapsuleComponent`) "None"))
    (set `self.X-RotationRate` (`KismetMathLibrary.MapRangeClamped` (.z _returnvalue_3) -360.0 360.0 -1.0 1.0))
    (set `self.Y-RotationRate` (`KismetMathLibrary.MapRangeClamped` (.y (`KismetMathLibrary.InverseTransformDirection` (`Actor.GetTransform` (`self.Character`)) _returnvalue_3)) -360.0 360.0 1.0 -1.0))
    (if (or (`self.DodgingLeft`) (`self.DodgingRight`))
      (`CharacterMovementComponent.AddForce` (`self.MovementComponent`) (* (select `bool` (`self.DodgingLeft`) :`false` _returnvalue_2 :`true` (* _returnvalue_2 -1.0)) (`self.DodgeCurrentForce`)))
      (set `self.DodgeCurrentForce` (`KismetMathLibrary.FInterpTo` (`self.DodgeCurrentForce`) 0.0 (`self.Delta`) 4.0)))
    (elif (!= _returnvalue_pitch 0.0)
      (`Actor.K2_SetActorRotation` (`self.Character`) (`KismetMathLibrary.RInterpTo` (`KismetMathLibrary.MakeRotator` _returnvalue_roll _returnvalue_pitch _returnvalue_yaw) (`KismetMathLibrary.MakeRotator` _returnvalue_roll 0.0 _returnvalue_yaw) (`self.Delta`) 8.0) false))))

(event `DodgeLeft`
  ;[0.599 1 0.6833] Left Dodge - set current dodge force equal to the default dodge force (applied during FlightUpdates). Dodge state ends after 1.5s. The 0.1s delay for the DoOnce ensures the AnimBP State machine moves out of the dodge state before being able to re-enter it.
  (if (`self.FastFlight`)
    (if (`KismetMathLibrary.BooleanNOR` (`self.DodgingLeft`) (`self.DodgingRight`))
      (`/Engine/EditorBlueprintResources/StandardMacros.DoOnce` false :!label _label
        (:`Completed`
          (set `self.DodgingLeft` true)
          (set `self.DodgeCurrentForce` (`self.DodgeForce`))
          (`KismetSystemLibrary.Delay` 1.5)
          (set `self.DodgingLeft` false)
          (`KismetSystemLibrary.Delay` 0.1)
          (goto _label :!via `Reset`))))))

(event `DodgeRight`
  ;[0.599 1 0.6833] Right Dodge - set current dodge force equal to the default dodge force (applied during FlightUpdates). Dodge state ends after 1.5s. The 0.1s delay for the DoOnce ensures the AnimBP State machine moves out of the dodge state before being able to re-enter it.
  (if (`self.FastFlight`)
    (if (`KismetMathLibrary.BooleanNOR` (`self.DodgingLeft`) (`self.DodgingRight`))
      (`/Engine/EditorBlueprintResources/StandardMacros.DoOnce` false :!label _label_2
        (:`Completed`
          (set `self.DodgingRight` true)
          (set `self.DodgeCurrentForce` (`self.DodgeForce`))
          (`KismetSystemLibrary.Delay` 1.5)
          (set `self.DodgingRight` false)
          (`KismetSystemLibrary.Delay` 0.1)
          (goto _label_2 :!via `Reset`))))))

(event `MoveUp`
  (params (AxisValue :type "Float (double-precision)"))
  ;[0.599 1 0.6833] Handle input for hovering up and down
  (if (`self.Hover`)
    (`Pawn.AddMovementInput` (`self.Character`) (0.0 0.0 1.0) AxisValue false)))

(fn `ToggleFastFlight`
  (bind _returnvalue (`KismetMathLibrary.MakeVector` (.x (`SceneComponent.K2_GetComponentLocation` (`self.CapsuleComponent`))) (.y (`SceneComponent.K2_GetComponentLocation` (`self.CapsuleComponent`))) (+ (- (.z (`SceneComponent.K2_GetComponentLocation` (`self.CapsuleComponent`))) (`self.CapsuleHalfHeight`)) (`self.CapsuleRadius`))))
  (bind _returnvalue_2 (`KismetMathLibrary.MakeVector` (.x (`SceneComponent.K2_GetComponentLocation` (`self.CapsuleComponent`))) (.y (`SceneComponent.K2_GetComponentLocation` (`self.CapsuleComponent`))) (- (+ (.z (`SceneComponent.K2_GetComponentLocation` (`self.CapsuleComponent`))) (`self.CapsuleHalfHeight`)) (`self.CapsuleRadius`))))
  ;[0.599 1 0.6833] Only continue if not currently groundslamming.
  (if (not (`self.GroundSlam`))
    ;[0.599 1 0.6833] Toggle FastFlight variable, branch depending on outcome
    (bind _output_get (set `self.FastFlight` (not (`self.FastFlight`))))
    (if _output_get
      ;[0.599 1 0.6833] If currently in Hover mode, toggle it off
      (if (`self.Hover`)
        (`self.ToggleHover`))
      ;[0.599 1 0.6833] Change flight speed and acceleration
      (set `CharacterMovementComponent.MaxFlySpeed` (`self.FastFlightSpeed`) (`self.MovementComponent`))
      (set `CharacterMovementComponent.MaxAcceleration` (`self.FastFlightAcceleration`) (`self.MovementComponent`))
      ;[0.599 1 0.6833] Change character movement modes
      (`CharacterMovementComponent.SetMovementMode` (`self.MovementComponent`) "MOVE_Flying" 0)
      (set `CharacterMovementComponent.bOrientRotationToMovement` false (`self.MovementComponent`))
      ;[0.599 1 0.6833] Shorten the capsule height while in flight mode to better match the horizontal character. Restore original height when exiting flight mode.
      (`CapsuleComponent.SetCapsuleHalfHeight` (`self.CapsuleComponent`) (`CapsuleComponent.GetUnscaledCapsuleRadius` (`self.CapsuleComponent`)) true)
      ;[0.599 1 0.6833] Record current max flight speed for use in the AnimBP
      (set `self.CurrentMaxFlySpeed` (`CharacterMovementComponent.MaxFlySpeed` (`self.MovementComponent`)))
      (else
        ;[0.599 1 0.6833] Before disabling FastFlight, perform two Capsule Traces to see if there's enough room immediately above or below the player to restore their full capsule size. If so, continue. If not, re-enable FastFlight.
        (bind (_outhit _returnvalue_3) (`KismetSystemLibrary.CapsuleTraceSingle` _returnvalue_2 (+ _returnvalue_2 (0.01 0.01 0.01)) (`self.CapsuleRadius`) (`self.CapsuleHalfHeight`) "TraceTypeQuery1"))
        (if _returnvalue_3
          (bind (_outhit_2 _returnvalue_4) (`KismetSystemLibrary.CapsuleTraceSingle` _returnvalue (- _returnvalue (0.01 0.01 0.01)) (`self.CapsuleRadius`) (`self.CapsuleHalfHeight`) "TraceTypeQuery1"))
          (if _returnvalue_4
            (set `self.FastFlight` true)
            (else
              ;[0.599 1 0.6833] Get Z-momentum to be applied when flight mode ends
              (bind _returnvalue_5 (`PrimitiveComponent.GetPhysicsLinearVelocity` (`self.CapsuleComponent`) "None" :!label _label))
              (set `self.Z-Momentum` (.z _returnvalue_5))
              (`CharacterMovementComponent.SetMovementMode` (`self.MovementComponent`) "MOVE_Walking" 0)
              (set `CharacterMovementComponent.bOrientRotationToMovement` true (`self.MovementComponent`))
              (`CapsuleComponent.SetCapsuleHalfHeight` (`self.CapsuleComponent`) (`self.CapsuleHalfHeight`) true)
              ;[0.599 1 0.6833] Clear both dodge states to cancel any in-progresses dodges.
              (set `self.DodgingLeft` false)
              (set `self.DodgingRight` false)
              ;[0.599 1 0.6833] If the character is no longer in either flight mode, add a portion of its previous Z-speed so that it doesn't lose all vertical momentum
              (if (`KismetMathLibrary.BooleanNOR` (`self.Hover`) (`self.FastFlight`))
                (`Character.LaunchCharacter` (`self.Character`) (`KismetMathLibrary.MakeVector` 0.0 0.0 (* (`self.Z-Momentum`) 0.7)) false true)
                ;[0.599 1 0.6833] Restore the character's original ground acceleration value.
                (set `CharacterMovementComponent.MaxAcceleration` (`self.DefaultAcceleration`) (`self.MovementComponent`)))))
          (else
            (goto _label)))))))

(fn `ToggleHover`
  ;[0.599 1 0.6833] Only continue if not currently groundslamming.
  (if (not (`self.GroundSlam`))
    ;[0.599 1 0.6833] Toggle Hover variable, branch depending on outcome
    (bind _output_get (set `self.Hover` (not (`self.Hover`))))
    (if _output_get
      ;[0.599 1 0.6833] If currently in Fast Flight mode, toggle it off
      (if (`self.FastFlight`)
        (`self.ToggleFastFlight`))
      ;[0.599 1 0.6833] Only proceed if Fast Flight was successfully disabled. Else, re-disable Hover.
      (if (`self.FastFlight`)
        (set `self.Hover` false)
        (else
          ;[0.599 1 0.6833] Change flight speed and acceleration
          (set `CharacterMovementComponent.MaxFlySpeed` (`self.HoverSpeed`) (`self.MovementComponent`))
          (set `CharacterMovementComponent.MaxAcceleration` (`self.HoverAcceleration`) (`self.MovementComponent`))
          ;[0.599 1 0.6833] Change character movement modes
          (`CharacterMovementComponent.SetMovementMode` (`self.MovementComponent`) "MOVE_Flying" 0)
          (set `CharacterMovementComponent.bOrientRotationToMovement` false (`self.MovementComponent`))
          ;[0.599 1 0.6833] Record current max flight speed for use in the AnimBP
          (set `self.CurrentMaxFlySpeed` (`CharacterMovementComponent.MaxFlySpeed` (`self.MovementComponent`)))))
      (else
        ;[0.599 1 0.6833] Get Z-momentum to be applied when flight mode ends
        (bind _returnvalue (`PrimitiveComponent.GetPhysicsLinearVelocity` (`self.CapsuleComponent`) "None"))
        (set `self.Z-Momentum` (.z _returnvalue))
        (`CharacterMovementComponent.SetMovementMode` (`self.MovementComponent`) "MOVE_Walking" 0)
        (set `CharacterMovementComponent.bOrientRotationToMovement` true (`self.MovementComponent`))
        ;[0.599 1 0.6833] If the character is no longer in either flight mode, add a portion of its previous Z-speed so that it doesn't lose all vertical momentum
        (if (`KismetMathLibrary.BooleanNOR` (`self.Hover`) (`self.FastFlight`))
          (`Character.LaunchCharacter` (`self.Character`) (`KismetMathLibrary.MakeVector` 0.0 0.0 (* (`self.Z-Momentum`) 0.7)) false true)
          ;[0.599 1 0.6833] Restore the character's original ground acceleration value.
          (set `CharacterMovementComponent.MaxAcceleration` (`self.DefaultAcceleration`) (`self.MovementComponent`)))))))

(fn `TriggerGroundSlam`
  ;[0.599 1 0.6833] Set GroundSlam to true for use in the AnimBP. Other logic for Ground Slam could be added here (i.e. dealing damage, etc)
  (set `self.GroundSlam` true)
  ;;[0.599 1 0.6833] Temporarily disable movement until ground slam ends
  (`Controller.SetIgnoreMoveInput` (`Pawn.GetController` (`self.Character`)) true))